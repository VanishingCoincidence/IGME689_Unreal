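; BP_FeaturePoint is an actor in the racing game that marks a geographic point on an ArcGIS map through its ArcGISLocation component.
; On BeginPlay it caches the ArcGIS map actor and pawn.
; UpdatePosition places it at a WGS84 longitude and latitude, snapped to the ground.
; SpawnFeaturePoints only repositions it, using absolute height and feeding Latitude into X and Longitude into Y, the reverse of UpdatePosition.
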(event EventBeginPlay
  (bind _returnvalue (Actor|GetActorOfClass "/Script/ArcGISMapsSDK.ArcGISMapActor"))
  (Variables|Default|SetArcGISMap _returnvalue)
  (bind _returnvalue_2 (Actor|GetActorOfClass "/Script/ArcGISSamples.ArcGISPawn"))
  (Variables|Default|SetPawn _returnvalue_2))

(event Collision|EventActorBeginOverlap
  (params (OtherActor :type Actor%20Object%20Reference)))

(event EventTick
  (params (DeltaSeconds :type Float%20%28single-precision%29)))

(fn ConstructionScript)

(fn UpdatePosition
  (params (Longitude :type Float%20%28double-precision%29) (Latitude :type Float%20%28double-precision%29))
  (bind _arcgislocation (Variables|Default|GetArcGISLocation))
  (bind _returnvalue (Class|ArcGISSpatialReference|WGS84))
  (bind _returnvalue_2 (Class|ArcGISPoint|CreateArcGISPointwithXYZSpatialReference Longitude Latitude 0.0 _returnvalue))
  (Class|ArcGISLocationComponent|SetPosition _arcgislocation _returnvalue_2)
  (Class|ArcGISLocationComponent|SetSurfacePlacementMode _arcgislocation "OnTheGround"))

(fn SpawnFeaturePoints
  (params (Latitude :type Float%20%28double-precision%29) (Longitude :type Float%20%28double-precision%29))
  (bind _arcgislocation (Variables|Default|GetArcGISLocation))
  (bind _returnvalue (Class|ArcGISSpatialReference|WGS84))
  (bind _returnvalue_2 (Class|ArcGISPoint|CreateArcGISPointwithXYZSpatialReference Latitude Longitude 0.0 _returnvalue))
  (Class|ArcGISLocationComponent|SetPosition _arcgislocation _returnvalue_2)
  (Class|ArcGISLocationComponent|SetSurfacePlacementMode _arcgislocation "AbsoluteHeight"))