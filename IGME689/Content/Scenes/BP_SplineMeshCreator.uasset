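; Actor that builds a spline-following mesh path from geographic coordinates on an ArcGIS map.
; BeginPlay caches the ArcGISMapActor, and PopulateSplines converts longitude, latitude and altitude to engine positions, inserting each as a spline point.
; AddMesh then adds a spline mesh component per segment, shaped by local point locations and tangents.
; The same loop sits disconnected in the construction script, so it never runs there.
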(event EventBeginPlay
  (bind _returnvalue (Actor|GetActorOfClass "/Script/ArcGISMapsSDK.ArcGISMapActor"))
  (Variables|Default|SetArcGISMap _returnvalue))

(fn ConstructionScript)

(fn PopulateSplines
  (params (Longitude :type Float%20%28double-precision%29) (Latitude :type Float%20%28double-precision%29) (Altitude :type Float%20%28double-precision%29) (Index :type Integer))
  (bind _returnvalue (Class|ArcGISPoint|CreateArcGISPointwithXYZ Longitude Latitude Altitude))
  (bind _returnvalue_2 (Class|ArcGISMapComponent|TransformPointtoEnginePosition (Variables|/Script/ArcGISMapsSDK.ArcGISMapActor|GetMapComponent (Variables|Default|GetArcGISMap)) _returnvalue))
  (Spline|AddSplinePointatIndex (Variables|Default|GetSpline) _returnvalue_2 Index "World" true)
  (return _returnvalue_2))

(fn AddMesh
  (bind _spline (Variables|Default|GetSpline))
  (for _index (range 0 (- (Spline|GetNumberOfSplinePoints (Variables|Default|GetSpline)) 2))
    (bind _returnvalue (AddComponent|AddSplineMeshComponent false))
    (SplineMesh|SetStartandEnd _returnvalue (.Location (Spline|GetLocationandTangentatSplinePoint _spline _index "Local")) (.Tangent (Spline|GetLocationandTangentatSplinePoint _spline _index "Local")) (.Location (Spline|GetLocationandTangentatSplinePoint _spline (+ _index 1) "Local")) (.Tangent (Spline|GetLocationandTangentatSplinePoint _spline (+ _index 1) "Local")) true :!class /Script/Engine.SplineMeshComponent)
    (Transformation|AttachComponentToComponent _returnvalue (Variables|Default|GetDefaultSceneRoot) "None" "KeepRelative" "KeepRelative" "KeepRelative" true)))