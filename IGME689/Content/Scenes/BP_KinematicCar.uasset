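; BP_KinematicCar is a player-driven car that moves kinematically, without physics forces.
; Throttle and Steer axes ease speed and steering angle toward scaled maximums with FInterpTo.
; Tick sweeps the actor along its right vector and yaws it in proportion to speed times steering angle.
; Look axes rotate the SpringArm, and BeginPlay caches the skeletal mesh's AnimBlueprint, which this graph never uses afterward.
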(event EventBeginPlay
  (bind _aslow_skeleton_anim_blueprint (Utilities|Casting|CastTolow_Skeleton_AnimBlueprint (Components|SkeletalMesh|GetAnimInstance (Variables|Default|GetSkeletalMesh))))
  (Variables|Default|SetAnimation _aslow_skeleton_anim_blueprint))

(event Collision|EventActorBeginOverlap
  (params (OtherActor :type Actor%20Object%20Reference)))

(event EventTick
  (params (DeltaSeconds :type Float%20%28single-precision%29))
  (bind _currentspeed (Variables|Default|GetCurrentSpeed))
  (Transformation|AddActorWorldOffset (* DeltaSeconds (* (Transformation|GetActorRightVector) _currentspeed)) true)
  (Class|Actor|AddActorWorldRotation (Math|Rotator|MakeRotator 0.0 0.0 (* _currentspeed (Variables|Default|GetCurrentSteeringAngle) (Variables|Default|GetSpeedToRot) (Utilities|Time|GetWorldDeltaSeconds)))))

(event Input|AxisEvents|InputAxisThrottle
  (params (AxisValue :type Float%20%28single-precision%29))
  (Variables|Default|SetCurrentSpeed (Math|Interpolation|FInterpTo (Variables|Default|GetCurrentSpeed) (* AxisValue (Variables|Default|GetMaxSpeed)) (Utilities|Time|GetWorldDeltaSeconds) 4.0)))

(event Input|AxisEvents|InputAxisSteer
  (params (AxisValue :type Float%20%28single-precision%29))
  (Variables|Default|SetCurrentSteeringAngle (Math|Interpolation|FInterpTo (Variables|Default|GetCurrentSteeringAngle) (* AxisValue (Variables|Default|GetMaxSteeringAngle)) (Utilities|Time|GetWorldDeltaSeconds) 4.0)))

(event Input|AxisEvents|InputAxisLookSide
  (params (AxisValue :type Float%20%28single-precision%29))
  (Transformation|AddRelativeRotation (Variables|Default|GetSpringArm) (Math|Rotator|MakeRotator 0.0 0.0 AxisValue) false false))

(event Input|AxisEvents|InputAxisLookUp
  (params (AxisValue :type Float%20%28single-precision%29))
  (Transformation|AddRelativeRotation (Variables|Default|GetSpringArm) (Math|Rotator|MakeRotator 0.0 AxisValue 0.0) false false))

(fn ConstructionScript)