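; BP_Spawner builds the Shanghai International Circuit as a spline mesh in an ArcGIS map from feature layer data.
; One second after BeginPlay, it filters the FeatureLayerQuery features by name and applies a fixed altitude offset.
; The first coordinate repositions the pawn and map origin, then spawns BP_SplineMeshCreator at the converted engine position.
; Every coordinate feeds that creator's PopulateSplines, and AddMesh finishes the track.
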(event Custom|AddItemsToList
  (bind _featurelayerquery (Variables|Default|GetFeatureLayerQuery))
  (Utilities|IsValid _featurelayerquery
    (:Is%20Valid
      (for _array_element (Variables|/Script/IGME689.FeatureLayerQuery|Getfeatures _featurelayerquery)
        (if (Utilities|Enum|Equal(Enum) (.name _array_element) "Shanghai International Circuit")
          (Variables|Default|SetAltitude (- (Math|Conversions|ToFloat(Integer) (.altitude _array_element)) 11.5))
          (for (_array_element_2 _array_index) (.geometries _array_element)
            (if (== _array_index 0)
              (CallFunction|ConfirmLocation (Utilities|Array|Get(acopy) (Utilities|Struct|BreakGeometries _array_element_2)) (Utilities|Array|Get(acopy) (Utilities|Struct|BreakGeometries _array_element_2) 1) (Variables|Default|GetAltitude))
              (Default|PopulateSplines (Variables|Default|GetSpline) (Utilities|Array|Get(acopy) (Utilities|Struct|BreakGeometries _array_element_2)) (Utilities|Array|Get(acopy) (Utilities|Struct|BreakGeometries _array_element_2) 1) (Variables|Default|GetAltitude) _array_index)
              (else
                (Default|PopulateSplines (Variables|Default|GetSpline) (Utilities|Array|Get(acopy) (Utilities|Struct|BreakGeometries _array_element_2)) (Utilities|Array|Get(acopy) (Utilities|Struct|BreakGeometries _array_element_2) 1) (Variables|Default|GetAltitude) _array_index))))
          (Default|AddMesh (Variables|Default|GetSpline)))))
    (:Is%20Not%20Valid
      (Development|PrintString "Not Valid"))))

(event Custom|ConfirmLocation
  (params (X :type Float%20%28double-precision%29) (Y :type Float%20%28double-precision%29) (Z :type Float%20%28double-precision%29))
  (bind _arcgismap (Variables|Default|GetArcGISMap))
  (bind _mapcomponent (Variables|/Script/ArcGISMapsSDK.ArcGISMapActor|GetMapComponent _arcgismap))
  (bind _returnvalue (Class|ArcGISSpatialReference|WGS84))
  (bind _returnvalue_2 (Class|ArcGISPoint|CreateArcGISPointwithXYZSpatialReference X Y Z _returnvalue))
  (Class|ArcGISLocationComponent|SetPosition (Actor|GetComponentbyClass (Variables|Default|GetPawn) "/Script/ArcGISMapsSDK.ArcGISLocationComponent") _returnvalue_2)
  (bind _returnvalue_3 (Class|ArcGISPoint|CreateArcGISPointwithXYZSpatialReference X Y Z _returnvalue))
  (Class|ArcGISMapComponent|SetOriginPosition _mapcomponent _returnvalue_3)
  (bind _returnvalue_4 (Class|ArcGISMapComponent|TransformPointtoEnginePosition _mapcomponent _returnvalue_3))
  (bind _returnvalue_5 (Game|SpawnActorfromClass "/Game/Scenes/BP_SplineMeshCreator.BP_SplineMeshCreator_C" (Math|Transform|MakeTransform _returnvalue_4 "0, 0, 0" "1.000000,1.000000,1.000000") "Undefined" "MultiplyWithRoot" 0 0))
  (bind _output_get (Variables|Default|SetSpline _returnvalue_5))
  (Spline|ClearSplinePoints (Variables|/Game/Scenes/BP_SplineMeshCreator.BP_SplineMeshCreator_C|GetSpline _output_get) true))

(event EventBeginPlay
  (bind _returnvalue (Actor|GetActorOfClass "/Script/IGME689.FeatureLayerQuery"))
  (Variables|Default|SetFeatureLayerQuery _returnvalue)
  (Utilities|FlowControl|Delay 1.0)
  (CallFunction|AddItemstoList)
  (bind _returnvalue_2 (Actor|GetActorOfClass "/Script/ArcGISMapsSDK.ArcGISMapActor"))
  (Variables|Default|SetArcGISMap _returnvalue_2)
  (bind _returnvalue_3 (Actor|GetActorOfClass "/Script/ArcGISSamples.ArcGISPawn"))
  (Variables|Default|SetPawn _returnvalue_3))

(fn ConstructionScript)